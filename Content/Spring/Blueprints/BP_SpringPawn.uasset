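; BP_SpringPawn is the player pawn, a character on two leg springs, handling movement, mouse look, sprint and a pause menu.
; Tick feeds the timer and speed to the HUD, samples speed history at fixed intervals and draws predicted trajectories from both springs.
; Landings play speed-scaled, randomized spring sounds, and faster movement lowers the move component's direction lerp.
; Hitting a goal actor shows a check on the HUD.
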(event EventTick
  (params (DeltaSeconds :type Float%20%28single-precision%29))
  (bind _returnvalue (Math|Random|RandomFloatinRange 0.5 0.8))
  (bind _returnvalue_2 (Math|Random|RandomFloatinRange 0.7 1.1))
  (bind _springcharacterlegspring (Variables|Default|GetSpringCharacterLegSpring))
  (bind _velocitysavedelta (Variables|Default|GetVelocitySaveDelta))
  (bind _movecomponent (Variables|Default|GetMoveComponent))
  (bind _movecomponent_2 (Variables|Default|GetMoveComponent))
  (bind _directionlerpmax (Variables|Default|GetDirectionLerpMax))
  (bind _velocity (Variables|/Script/Engine.MovementComponent|GetVelocity _movecomponent))
  (bind _returnvalue_3 (Math|Vector|VectorLength _velocity))
  (bind _returnvalue_4 (/ _returnvalue_3 4e+03))
  (bind _returnvalue_5 (- 1.0 _returnvalue_4))
  (bind _returnvalue_6 (* _returnvalue _returnvalue_4))
  (bind _returnvalue_7 (Math|Float|Clamp(Float) _returnvalue_6 0.2 0.7))
  (bind _returnvalue_8 (* _returnvalue_2 _returnvalue_5))
  (bind _returnvalue_9 (Math|Float|Clamp(Float) _returnvalue_8 0.8 1.3))
  (Utilities|FlowControl|Sequence
    (:then_0
      (Default|UpdatefromTimer (Variables|Default|GetPlayerHUD) (Variables|Default|GetTimerComponent))
      (bind _output_get (Variables|Default|SetVelocitySaveAccumulator (+ (Variables|Default|GetVelocitySaveAccumulator) DeltaSeconds)))
      (for _index (range 0 (Math|Float|Floor (/ _output_get _velocitysavedelta)))
        (Variables|Default|SetVelocitySaveAccumulator (- (Variables|Default|GetVelocitySaveAccumulator) _velocitysavedelta))
        (Utilities|Array|Add (Variables|Default|GetVelocityArray) (Math|Vector|VectorLength (Variables|/Script/Engine.MovementComponent|GetVelocity (Variables|Default|GetMoveComponent)))))
      (Variables|/Game/Spring/Interface/HUD.HUD_C|SetDisplayVelocity (Variables|Default|GetPlayerHUD) (/ (Math|Vector|VectorLength (Variables|/Script/Engine.MovementComponent|GetVelocity (Variables|Default|GetMoveComponent))) 1e+02)))
    (:then_1
      (Class|SpringPawnMovementComponent|DrawTrajectory (Variables|Default|GetMoveComponent) 2.0 0.05 (Math|Vector|RotateVector (Variables|/Script/Engine.SceneComponent|GetRelativeLocation (Variables|Default|GetSpringCharacterLegSpring)) (Transformation|GetActorRotation)))
      (Class|SpringPawnMovementComponent|DrawTrajectory (Variables|Default|GetMoveComponent) 2.0 0.05 (Math|Vector|RotateVector (Variables|/Script/Engine.SceneComponent|GetRelativeLocation (Variables|Default|GetSpringCharacterLegSpring1)) (Transformation|GetActorRotation))))
    (:then_2
      (if (Variables|/Script/Spring.SpringPawnMovementComponent|GetHitGroundLastFrame (Variables|Default|GetMoveComponent))
        (if (Variables|/Script/Spring.SpringCharacterLegSpring|GetGrounded _springcharacterlegspring)
          (Audio|PlaySoundatLocation "/Game/Spring/Assets/Sounds/Spring_Electric_Force.Spring_Electric_Force" (Variables|/Script/Spring.SpringCharacterLegSpring|GetGroundedLocation _springcharacterlegspring) "0, 0, 0" _returnvalue_7 _returnvalue_9)
          (else
            (Audio|PlaySoundatLocation "/Game/Spring/Assets/Sounds/Spring_Electric_Force.Spring_Electric_Force" (Variables|/Script/Spring.SpringCharacterLegSpring|GetGroundedLocation (Variables|Default|GetSpringCharacterLegSpring1)) "0, 0, 0" _returnvalue_7 _returnvalue_9)))))
    (:then_3
      (Variables|/Script/Spring.SpringPawnMovementComponent|SetDirectionLerpValue _movecomponent_2 (Math|Float|Clamp(Float) (- _directionlerpmax (Math|Float|Square (/ (Math|Vector|VectorLength (Variables|/Script/Engine.MovementComponent|GetVelocity _movecomponent_2)) 4e+03))) (Variables|Default|GetDirectionLerpMin) _directionlerpmax)))))

(event EventBeginPlay
  (bind _returnvalue (Game|GetPlayerController 0))
  (Utilities|FlowControl|Sequence
    (:then_0
      ;[1 1 1] We probably want to change this...
      (bind _returnvalue_2 (UserInterface|CreateWidget "/Game/Spring/Interface/HUD.HUD_C"))
      (bind _output_get (Variables|Default|SetPlayerHUD _returnvalue_2))
      (UserInterface|Viewport|AddtoViewport _output_get 0)
      (Input|SetInputModeGameOnly _returnvalue)
      (AddComponent|AddChildActorComponent _returnvalue false))))

(event Collision|EventHit
  (params (MyComp :type Primitive%20Component%20Object%20Reference) (Other :type Actor%20Object%20Reference) (OtherComp :type Primitive%20Component%20Object%20Reference) (bSelfMoved :type Boolean) (HitLocation :type Vector :default "0, 0, 0") (HitNormal :type Vector :default "0, 0, 0") (NormalImpulse :type Vector :default "0, 0, 0") (Hit :type Hit%20Result%20Structure%20%28by%20ref%29))
  (CallFunction|CheckWon Hit))

(event Input|ActionEvents|InputActionSprint
  (params (Key :type Key%20Structure :default "AnyKey"))
  (bind _movecomponent (Variables|Default|GetMoveComponent))
  (:Pressed
    (Class|SpringPawnMovementComponent|SetSprint _movecomponent true))
  (:Released
    (Class|SpringPawnMovementComponent|SetSprint _movecomponent false)))

(event Input|ActionEvents|InputActionPause
  (params (Key :type Key%20Structure :default "AnyKey"))
  ;[1 1 1] We probably want to change this...
  (:Pressed
    (Utilities|IsValid (Variables|Default|GetPlayerPauseMenu)
      (:Is%20Valid
        _)
      (:Is%20Not%20Valid
        (bind _returnvalue (UserInterface|CreateWidget "/Game/Spring/Interface/PauseMenu.PauseMenu_C"))
        (Variables|Default|SetPlayerPauseMenu _returnvalue)))
    (Input|SetInputModeUIOnly (Game|GetPlayerController 0) (Variables|Default|GetPlayerPauseMenu) false)
    (UserInterface|Viewport|AddtoViewport (Variables|Default|GetPlayerPauseMenu) 0)
    (Game|SetGamePaused true)))

(event Input|AxisEvents|InputAxisForwardAxis
  (params (AxisValue :type Float%20%28single-precision%29))
  (Pawn|Input|AddMovementInput (Transformation|GetActorForwardVector) AxisValue false))

(event Input|AxisEvents|InputAxisLookUp
  (params (AxisValue :type Float%20%28single-precision%29))
  (bind _playercamera (Variables|Default|GetPlayerCamera))
  (bind _returnvalue (Transformation|GetWorldRotation _playercamera))
  (bind (_roll _pitch _yaw) (Math|Rotator|BreakRotator _returnvalue))
  (Transformation|SetWorldRotation _playercamera (Math|Rotator|MakeRotator _roll (Math|Float|ClampAngle (+ (* AxisValue -1.0) _pitch) -89.0 89.0) _yaw) false false))

(event Input|AxisEvents|InputAxisLookRight
  (params (AxisValue :type Float%20%28single-precision%29))
  (Pawn|Input|AddControllerYawInput AxisValue))

(event Input|AxisEvents|InputAxisRightAxis
  (params (AxisValue :type Float%20%28single-precision%29))
  (Pawn|Input|AddMovementInput (Transformation|GetActorRightVector) AxisValue false))

(fn ConstructionScript)

(fn CheckWon
  (params (Hit :type Hit%20Result%20Structure))
  (if (== (Utilities|GetClass (.HitActor (Collision|BreakHitResult Hit))) "/Game/Spring/Blueprints/Asset_blueprints/Goal_blueprint.Goal_blueprint_C")
    (Default|ShowCheck (Variables|Default|GetPlayerHUD))))
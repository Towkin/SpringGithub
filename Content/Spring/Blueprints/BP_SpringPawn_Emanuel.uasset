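; BP_SpringPawn_Emanuel is a first-person style player pawn with walking, sprinting and mouse-look input.
; Movement axes feed AddMovementInput along the actor's forward and right vectors, and the Sprint action toggles sprint on MoveComponent.
; Horizontal look adds controller yaw, while vertical look rotates PlayerCamera's world pitch directly, inverted and clamped just short of straight up and down.
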(event Input|ActionEvents|InputActionSprint
  (params (Key :type Key%20Structure :default "AnyKey"))
  (bind _movecomponent (Variables|Default|GetMoveComponent))
  (:Pressed
    (Class|SpringPawnMovementComponent|SetSprint _movecomponent true))
  (:Released
    (Class|SpringPawnMovementComponent|SetSprint _movecomponent false)))

(event Input|AxisEvents|InputAxisForwardAxis
  (params (AxisValue :type Float%20%28single-precision%29))
  (Pawn|Input|AddMovementInput (Transformation|GetActorForwardVector) AxisValue false))

(event Input|AxisEvents|InputAxisLookUp
  (params (AxisValue :type Float%20%28single-precision%29))
  (bind _playercamera (Variables|Default|GetPlayerCamera))
  (bind _returnvalue (Transformation|GetWorldRotation _playercamera))
  (bind (_roll _pitch _yaw) (Math|Rotator|BreakRotator _returnvalue))
  (Transformation|SetWorldRotation _playercamera (Math|Rotator|MakeRotator _roll (Math|Float|ClampAngle (+ (* AxisValue -1.0) _pitch) -89.0 89.0) _yaw) false false))

(event Input|AxisEvents|InputAxisLookRight
  (params (AxisValue :type Float%20%28single-precision%29))
  (Pawn|Input|AddControllerYawInput AxisValue))

(event Input|AxisEvents|InputAxisRightAxis
  (params (AxisValue :type Float%20%28single-precision%29))
  (Pawn|Input|AddMovementInput (Transformation|GetActorRightVector) AxisValue false))

(fn ConstructionScript)
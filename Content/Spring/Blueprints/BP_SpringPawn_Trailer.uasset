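; BP_SpringPawn_Trailer is a player pawn with sprint, movement and look input, plus a pause action that opens a cached menu and pauses the game.
; Tick has MoveComponent draw predicted trajectories from both leg springs, offset by actor rotation.
; Yaw goes through the controller, while pitch rotates PlayerCamera directly with a clamp.
; The HUD is created but never added to the viewport, and the goal-hit check has no outcome.
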(event EventTick
  (params (DeltaSeconds :type Float%20%28single-precision%29))
  (Utilities|FlowControl|Sequence
    (:then_1
      (Class|SpringPawnMovementComponent|DrawTrajectory (Variables|Default|GetMoveComponent) 2.0 0.05 (Math|Vector|RotateVector (Variables|/Script/Engine.SceneComponent|GetRelativeLocation (Variables|Default|GetSpringCharacterLegSpring)) (Transformation|GetActorRotation)))
      (Class|SpringPawnMovementComponent|DrawTrajectory (Variables|Default|GetMoveComponent) 2.0 0.05 (Math|Vector|RotateVector (Variables|/Script/Engine.SceneComponent|GetRelativeLocation (Variables|Default|GetSpringCharacterLegSpring1)) (Transformation|GetActorRotation))))))

(event EventBeginPlay
  (Utilities|FlowControl|Sequence
    (:then_0
      ;[1 1 1] We probably want to change this...
      (UserInterface|CreateWidget "/Game/Spring/Interface/HUD.HUD_C"))))

(event Collision|EventHit
  (params (MyComp :type Primitive%20Component%20Object%20Reference) (Other :type Actor%20Object%20Reference) (OtherComp :type Primitive%20Component%20Object%20Reference) (bSelfMoved :type Boolean) (HitLocation :type Vector :default "0, 0, 0") (HitNormal :type Vector :default "0, 0, 0") (NormalImpulse :type Vector :default "0, 0, 0") (Hit :type Hit%20Result%20Structure%20%28by%20ref%29))
  (CallFunction|CheckWon Hit))

(event Input|ActionEvents|InputActionSprint
  (params (Key :type Key%20Structure :default "AnyKey"))
  (bind _movecomponent (Variables|Default|GetMoveComponent))
  (:Pressed
    (Class|SpringPawnMovementComponent|SetSprint _movecomponent true))
  (:Released
    (Class|SpringPawnMovementComponent|SetSprint _movecomponent false)))

(event Input|ActionEvents|InputActionPause
  (params (Key :type Key%20Structure :default "AnyKey"))
  ;[1 1 1] We probably want to change this...
  (:Pressed
    (Utilities|IsValid (Variables|Default|GetPlayerPauseMenu)
      (:Is%20Valid
        _)
      (:Is%20Not%20Valid
        (bind _returnvalue (UserInterface|CreateWidget "/Game/Spring/Interface/PauseMenu.PauseMenu_C"))
        (Variables|Default|SetPlayerPauseMenu _returnvalue)))
    (Input|SetInputModeUIOnly (Game|GetPlayerController 0) (Variables|Default|GetPlayerPauseMenu) false)
    (UserInterface|Viewport|AddtoViewport (Variables|Default|GetPlayerPauseMenu) 0)
    (Game|SetGamePaused true)))

(event Input|AxisEvents|InputAxisForwardAxis
  (params (AxisValue :type Float%20%28single-precision%29))
  (Pawn|Input|AddMovementInput (Transformation|GetActorForwardVector) AxisValue false))

(event Input|AxisEvents|InputAxisLookUp
  (params (AxisValue :type Float%20%28single-precision%29))
  (bind _playercamera (Variables|Default|GetPlayerCamera))
  (bind _returnvalue (Transformation|GetWorldRotation _playercamera))
  (bind (_roll _pitch _yaw) (Math|Rotator|BreakRotator _returnvalue))
  (Transformation|SetWorldRotation _playercamera (Math|Rotator|MakeRotator _roll (Math|Float|ClampAngle (+ (* AxisValue -1.0) _pitch) -89.0 89.0) _yaw) false false))

(event Input|AxisEvents|InputAxisLookRight
  (params (AxisValue :type Float%20%28single-precision%29))
  (Pawn|Input|AddControllerYawInput AxisValue))

(event Input|AxisEvents|InputAxisRightAxis
  (params (AxisValue :type Float%20%28single-precision%29))
  (Pawn|Input|AddMovementInput (Transformation|GetActorRightVector) AxisValue false))

(event Input|KeyboardEvents|SpaceBar
  (params (Key :type Key%20Structure :default "AnyKey")))

(fn ConstructionScript)

(fn CheckWon
  (params (Hit :type Hit%20Result%20Structure))
  (if (== (Utilities|GetClass (.HitActor (Collision|BreakHitResult Hit))) "/Game/Spring/Blueprints/Asset_blueprints/Goal_blueprint.Goal_blueprint_C")
    _))
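; Game instance that manages background music, starting the menu song on Init.
; PlayMusic replaces the current 2D audio component, and a finished-audio event plays the queued NextSong and requests another from GetRandomSong.
; ChangeMusic queues a song and sets fade-out timer state, though nothing here ticks that timer.
; GetRandomSong's random pick from DefaultSongList is left unconnected, so it returns no chosen song.
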(event OnAudioFinished(CurrentSong)
  (CallFunction|PlayMusic (Variables|Default|GetNextSong))
  (Variables|Default|SetNextSong (Utilities|GetRandomSong)))

(event EventInit
  (Utilities|FlowControl|Sequence
    (:then_0
      (Variables|Default|SetNextSong (Utilities|GetRandomSong))
      (CallFunction|PlayMusic (Variables|Default|GetMenuSong)))))

(fn PlayMusic
  (params (Song :type Sound%20Wave%20Object%20Reference))
  (Audio|Components|Audio|Stop (Variables|Default|GetCurrentSong))
  (bind _returnvalue (Audio|SpawnSound2D Song))
  (Variables|Default|SetCurrentSong _returnvalue)
  (Variables|Default|SetFadeOut false))

(fn ChangeMusic
  (params (NewSong :type Sound%20Wave%20Object%20Reference) (FadeTime :type Float%20%28single-precision%29))
  (Variables|Default|SetNextSong NewSong)
  (bind _output_get (Variables|Default|SetFadeTimerMax FadeTime))
  (Variables|Default|SetFadeTimer _output_get)
  (Variables|Default|SetFadeOut true))
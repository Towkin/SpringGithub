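; SpringMusicHandler manages 2D music playback for the menu and gameplay.
; PlayMenuMusic and PlayGameMusic feed MenuSong or the GetRandomSong result into PlayMusic, which stops and destroys the current song before spawning the next.
; GetRandomSong holds a random pick from DefaultSongList that is marked unused and, as written, excludes the last entry.
; EndPlay kills the music, and FadeOut is only reset, with no fade logic here.
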(event EventBeginPlay)

(event EventTick
  (params (DeltaSeconds :type Float%20%28single-precision%29)))

(event EventEndPlay
  (params (EndPlayReason :type EEndPlayReason%20Enum :default "Destroyed"))
  (CallFunction|KillMusic))

(fn PlayMusic
  (params (NewSong :type Sound%20Wave%20Object%20Reference))
  (CallFunction|KillMusic)
  (bind _returnvalue (Audio|SpawnSound2D NewSong))
  (Variables|Default|SetCurrentSong _returnvalue)
  (Variables|Default|SetFadeOut false))

(fn KillMusic
  (bind _currentsong (Variables|Default|GetCurrentSong))
  (Utilities|IsValid _currentsong
    (:Is%20Valid
      (Audio|Components|Audio|Stop _currentsong)
      (Components|DestroyComponent _currentsong))))

(fn PlayMenuMusic
  (CallFunction|PlayMusic (Variables|Default|GetMenuSong)))

(fn PlayGameMusic
  (CallFunction|PlayMusic (Utilities|GetRandomSong)))